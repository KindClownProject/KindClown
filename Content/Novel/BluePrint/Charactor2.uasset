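; Visual novel actor for character slot 2, showing Yukari, Maki, Akane or Aoi as the dialogue advances.
; Each Tick, while the game instance's Next flag is set, it moves to a base position and reveals the component matching the current Progress entry's Name if its Location is 2.
; After a match, a short Delay precedes clearing Next and shifting the actor along X; nothing here hides characters again.
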(event `self.ReceiveTick`
  (params (DeltaSeconds :type "Float (single-precision)"))
  (bind _asgroval_var (cast `/Game/Novel/Groval_var` (`GameplayStatics.GetGameInstance`)))
  (if (`/Game/Novel/Groval_var.Next` _asgroval_var)
    (`self.K2_SetActorLocation` (0.0 -100.0 0.0))
    (bind _progress (`/Game/Novel/Groval_var.Progress` _asgroval_var))
    (bind _output (`|GetArrayItem` (`/Game/Novel/Groval_var.Name` _asgroval_var) _progress))
    (bind _returnvalue (== (`|GetArrayItem` (`/Game/Novel/Groval_var.Location` _asgroval_var) _progress) 2))
    (if (and (`KismetStringLibrary.EqualEqual_StrStr` _output "Yukari") _returnvalue)
      (`SceneComponent.SetVisibility` (`self.Yukari`) true false)
      (`KismetSystemLibrary.Delay` 0.05 :!label _label)
      (set `/Game/Novel/Groval_var.Next` false _asgroval_var)
      (`self.K2_SetActorLocation` (-20.0 -100.0 0.0))
      (elif (and (`KismetStringLibrary.EqualEqual_StrStr` _output "Maki") _returnvalue)
        (`SceneComponent.SetVisibility` (`self.Maki`) true false)
        (goto _label)
        (elif (and (`KismetStringLibrary.EqualEqual_StrStr` _output "Akane") _returnvalue)
          (`SceneComponent.SetVisibility` (`self.Akane`) true false)
          (goto _label)
          (elif (and (`KismetStringLibrary.EqualEqual_StrStr` _output "Aoi") _returnvalue)
            (`SceneComponent.SetVisibility` (`self.Aoi`) true false)
            (goto _label)))))))

(fn `UserConstructionScript`)