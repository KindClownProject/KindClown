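; Player character Blueprint for KIndClown with camera-relative movement, mouse look, jumping and a chargeable magic shot.
; Holding MagicShot accumulates a capped charge on Tick, which also prints the value as debug text.
; Release spawns a TestBullet ahead of the actor, larger at full charge, and spends MP; insufficient charge fires nothing.
; AnyDamage subtracts from HP, with no death handling.
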(event `InputAction|MagicShot`
  (params (Key :type "Key Structure" :default "AnyKey"))
  (bind _chargetime (`self.ChargeTime`))
  ;[1 1 1] 魔弾発射
  (:`Pressed`
    (set `self.ChargeStart` true)
    (set `self.ChargeTime` 0.0 :!label _label))
  (:`Released`
    (set `self.ChargeStart` false)
    (if (and (>= _chargetime 5.0) (< _chargetime 10.0))
      (bind _output_get (set `self.ChargeScale` (1.0 1.0 1.0)))
      (`self.MagicShot` _output_get)
      (goto _label)
      (elif (== (`self.ChargeTime`) 10.0)
        (bind _output_get_2 (set `self.ChargeScale` (2.0 2.0 2.0)))
        (`self.MagicShot` _output_get_2)
        (goto _label)))))

(event `InputAxis|Turn` :overrideparent false
  (params (AxisValue :type "Float (single-precision)"))
  ;[1 1 1] マウス入力
  (`self.AddControllerYawInput` AxisValue))

(event `InputAction|Jump` :overrideparent false
  (params (Key :type "Key Structure" :default "AnyKey"))
  ;[1 1 1] ジャンプ
  (:`Pressed`
    (`self.Jump`))
  (:`Released`
    (`self.StopJumping`)))

(event `InputAction|Jump` :overrideparent false
  (params (Key :type "Key Structure" :default "AnyKey"))
  ;[1 1 1] ジャンプ
  (:`Pressed`
    (`self.Jump`))
  (:`Released`
    (`self.StopJumping`)))

(event `InputAxis|LookUp` :overrideparent false
  (params (AxisValue :type "Float (single-precision)"))
  ;[1 1 1] マウス入力
  (`self.AddControllerPitchInput` AxisValue))

(event `self.ReceiveTick`
  (params (DeltaSeconds :type "Float (single-precision)"))
  ;[1 1 1] 魔弾発射
  (`self.Charge` DeltaSeconds)
  (`KismetSystemLibrary.PrintString` (`KismetStringLibrary.Conv_DoubleToString` (`self.ChargeTime`)) true true (struct :`G` 0.66 :`B` 1.0 :`A` 1.0) 0.01))

(event `InputAxis|MoveForward` :overrideparent false
  (params (AxisValue :type "Float (single-precision)"))
  ;[1 1 1] 移動
  (`self.AddMovementInput` (`KismetMathLibrary.GetForwardVector` (`KismetMathLibrary.MakeRotator` 0.0 0.0 (.yaw (`self.GetControlRotation`)))) AxisValue))

(event `Charge`
  (params (Deltatime :type "Float (double-precision)"))
  ;[1 1 1] 魔弾発射
  (if (`self.ChargeStart`)
    (bind _output_get (set `self.ChargeTime` (+ (`self.ChargeTime`) Deltatime)))
    (if (>= _output_get 10.0)
      (set `self.ChargeTime` 10.0))))

(event `self.ReceiveAnyDamage`
  (params (Damage :type "Float (single-precision)") (DamageType :type "DamageType Object Reference") (InstigatedBy :type "Controller Object Reference") (DamageCauser :type "Actor Object Reference"))
  ;[1 1 1] HP(ダメージ設定)
  (set `self.HP` (- (`self.HP`) Damage)))

(event `InputAxis|MoveRight` :overrideparent false
  (params (AxisValue :type "Float (single-precision)"))
  ;[1 1 1] 移動
  (`self.AddMovementInput` (`KismetMathLibrary.GetRightVector` (`KismetMathLibrary.MakeRotator` 0.0 0.0 (.yaw (`self.GetControlRotation`)))) AxisValue))

(fn `MagicShot`
  (params (Scale :type "Vector Structure"))
  (bind _returnvalue (`self.K2_GetActorRotation`))
  (`|SpawnActorFromClass` "/Game/BluePrint/TestBullet.TestBullet_C" (`KismetMathLibrary.MakeTransform` (+ (* (`KismetMathLibrary.GetForwardVector` _returnvalue) 100.0) (`self.K2_GetActorLocation`)) _returnvalue Scale) "Undefined" "OverrideRootScale")
  (set `self.MP` (- (`self.MP`) 1.0))
  (return))

(fn `UserConstructionScript`)